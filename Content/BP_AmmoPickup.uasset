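; BP_AmmoPickup is an ammo pickup actor that refills the first-person character's AmmoInv.
; Overlapping Box1 with that character shows a widget and prints a debug "Hello", and leaving hides the widget.
; The PickUp event, not called within this Blueprint, adds a fixed amount to player 0's ammo up to a hard-coded cap, then destroys the actor.
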(event `/Game/BPI_PickUp.PickUp`
  (bind _asbp_first_person_character (cast `/Game/FirstPerson/Blueprints/BP_FirstPersonCharacter` (`GameplayStatics.GetPlayerCharacter` 0)))
  (if (> (- 18 (`/Game/FirstPerson/Blueprints/BP_FirstPersonCharacter.AmmoInv` _asbp_first_person_character)) 10)
    (set `/Game/FirstPerson/Blueprints/BP_FirstPersonCharacter.AmmoInv` (+ (`/Game/FirstPerson/Blueprints/BP_FirstPersonCharacter.AmmoInv` _asbp_first_person_character) 10) _asbp_first_person_character)
    (else
      (set `/Game/FirstPerson/Blueprints/BP_FirstPersonCharacter.AmmoInv` 18 _asbp_first_person_character)))
  (`self.K2_DestroyActor`))

(event `self.Box1.OnComponentBeginOverlap`
  (params (OverlappedComponent :type "PrimitiveComponent Object Reference") (OtherActor :type "Actor Object Reference") (OtherComp :type "PrimitiveComponent Object Reference") (OtherBodyIndex :type Integer) (bFromSweep :type Boolean) (SweepResult :type "HitResult Structure (by ref)"))
  (cast `/Game/FirstPerson/Blueprints/BP_FirstPersonCharacter` OtherActor)
  (`SceneComponent.SetVisibility` (`self.Widget`) true false)
  (`KismetSystemLibrary.PrintString` "Hello"))

(event `self.Box1.OnComponentEndOverlap`
  (params (OverlappedComponent :type "PrimitiveComponent Object Reference") (OtherActor :type "Actor Object Reference") (OtherComp :type "PrimitiveComponent Object Reference") (OtherBodyIndex :type Integer))
  (cast `/Game/FirstPerson/Blueprints/BP_FirstPersonCharacter` OtherActor)
  (`SceneComponent.SetVisibility` (`self.Widget`) false false))

(fn `UserConstructionScript`)